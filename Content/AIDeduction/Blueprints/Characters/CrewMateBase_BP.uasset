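; Base AI crewmate character for a social-deduction simulation, with an optional killer role that shows a weapon.
; Sight perception forwards seen and lost crewmates to a knowledge update, while a two-second loop attempts to forget observations during active play.
; A camera-facing widget displays task progress, and pause or resume toggles walk speed.
; Death swaps material, disables perception and spawns an initialized DeadCrewmate_BP; revival restores material and perception.
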(event `self.GetTaskProgressBar`
  ;[0.224 0.1399 0.1422] Initially grabbing the task progress bar.
  (bind _astask_progress_bar (cast `/Game/AIDeduction/Blueprints/UI/TaskProgressBar` (`WidgetComponent.GetUserWidgetObject` (`self.TaskBar`))))
  (bind _output_get (set `self.TaskProgressBar` _astask_progress_bar))
  (`Widget.SetVisibility` _output_get "Collapsed")
  ;[0.3943 1 0] Setting Weapon visibility and grabbing initial movement speed.
  (if (`self._isKiller`)
    (`SceneComponent.SetVisibility` (`self.Weapon`) true false))
  (set `self.InitialSpeed` (`CharacterMovementComponent.MaxWalkSpeed` (`self.CharacterMovement`))))

(event `self.ReceiveTick`
  (params (DeltaSeconds :type "Float (single-precision)"))
  ;[0.224 0.1399 0.1422] Make progress bar always face towards camera.
  (`SceneComponent.K2_SetWorldRotation` (`self.TaskBar`) (`KismetMathLibrary.FindLookAtRotation` (`SceneComponent.K2_GetComponentLocation` (`self.TaskBar`)) (`PlayerCameraManager.GetCameraLocation` (`PlayerController.PlayerCameraManager` (`GameplayStatics.GetPlayerController` 0)))) false false))

(event `self.AIPerception.OnTargetPerceptionUpdated`
  (params (Actor :type "Actor Object Reference") (Stimulus :type "AIStimulus Structure"))
  ;[0.3943 1 0] Performs function whenever a crew is seen or leaves view.
  (`self.OnSeenCrewmateUpdate` Actor (`.bSuccessfullySensed` (break `AIStimulus` Stimulus))))

(event `self.StartTask`
  (params (timeToCompleteTask :type "Float (single-precision)"))
  (bind _taskprogressbar (`self.TaskProgressBar`))
  ;[0.224 0.1399 0.1422] Starting and restarting the task progress bar.
  (set `/Game/AIDeduction/Blueprints/UI/TaskProgressBar.TotalTimeForTask` timeToCompleteTask _taskprogressbar)
  (`Widget.SetVisibility` _taskprogressbar "Visible"))

(event `self.ResetTaskProgress`
  (bind _taskprogressbar (`self.TaskProgressBar`))
  ;[0.224 0.1399 0.1422] Starting and restarting the task progress bar.
  (`Widget.SetVisibility` _taskprogressbar "Collapsed")
  (`ProgressBar.SetPercent` (`/Game/AIDeduction/Blueprints/UI/TaskProgressBar.TheProgressBar` _taskprogressbar) 0.0))

(event `self.StartPerception`
  ;[0.3943 1 0] Set perception capabilities on and off based on starting or ending a simulation.
  (`AIPerceptionStimuliSourceComponent.RegisterWithPerceptionSystem` (`self.AIPerceptionStimuliSource`))
  (`AIPerceptionComponent.SetSenseEnabled` (`self.AIPerception`) "/Script/AIModule.AISense_Sight" true))

(event `self.ResetPerception`
  (bind _aiperception (`self.AIPerception`))
  ;[0.3943 1 0] Set perception capabilities on and off based on starting or ending a simulation.
  (`AIPerceptionComponent.ForgetAll` _aiperception)
  (`AIPerceptionComponent.SetSenseEnabled` _aiperception "/Script/AIModule.AISense_Sight" false)
  (`AIPerceptionStimuliSourceComponent.UnregisterFromPerceptionSystem` (`self.AIPerceptionStimuliSource`)))

(event `self.InitializeMemorySystem`
  (bind __aideductiongamemode (`self._aiDeductionGameMode`))
  ;[1 0.06771 0.06771] Perform the memory system loop.
  (`KismetSystemLibrary.Delay` 2.0 :!label _label)
  (if (and (> (`KismetArrayLibrary.Array_Length` (`self._observedKnowledge`)) 0) (`AIDeductionGameMode._gameStarted` __aideductiongamemode) (not (`AIDeductionGameMode._gamePaused` __aideductiongamemode)) (not (`AIDeductionGameMode._victoryReached` __aideductiongamemode)) (`self.IsAlive`))
    (`self.AttemptToForget`)
    (goto _label)
    (else
      (goto _label))))

(event `self.Revive`
  ;[0.3943 1 0] Kill or revive the crewmate. Mostly just make the crewmate change colors at the moment. - Coleman.
  (`PrimitiveComponent.SetMaterial` (`self.Mesh`) 0 (`self.AliveMaterial`))
  (`self.StartPerception`)
  (set `self.IsAlive` true))

(event `self.Die`
  ;[0.3943 1 0] Kill or revive the crewmate. Mostly just make the crewmate change colors at the moment. - Coleman.
  (`|ExecutionSequence`
    (:`then_0`
      (`PrimitiveComponent.SetMaterial` (`self.Mesh`) 0 (`self.DeadMaterial`)))
    (:`then_1`
      (`self.ResetPerception`)
      (`self.ResetTaskProgress`)
      (set `self.IsAlive` false))
    (:`then_2`
      (bind _returnvalue (`|SpawnActorFromClass` "/Game/AIDeduction/Blueprints/Characters/DeadCrewmate_BP.DeadCrewmate_BP_C" (`self.GetTransform`) "AdjustIfPossibleButAlwaysSpawn" "OverrideRootScale" null null))
      (`DeadCrewmate.Initialize` _returnvalue (`self._name`) (`self._crewmateInformation`)))))

(event `self.Pause`
  ;[0.3943 1 0] Pause and Unpause Crewmate Movement.
  (set `CharacterMovementComponent.MaxWalkSpeed` 0.0 (`self.CharacterMovement`)))

(event `self.Resume`
  ;[0.3943 1 0] Pause and Unpause Crewmate Movement.
  (set `CharacterMovementComponent.MaxWalkSpeed` (`self.InitialSpeed`) (`self.CharacterMovement`)))

(fn `UserConstructionScript`)